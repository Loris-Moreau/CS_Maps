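; Time remapping sequence actor that scrubs ActiveSequence to a set PlaybackTime or PlaybackFrame, with frame and marked-frame stepping.
; Each update turns playback change per delta second into absolute time dilation for listed or class-gathered actors and their Niagara and Cascade components.
; It optionally feeds playback time to materials through a parameter collection.
; On sequence change it deactivates camera cuts and TimeController subsections; destruction resets dilation and the material override.
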(event `self.ReceiveDestroyed`
  (`self.ResetParticlesAndMaterials`)
  (`KismetSystemLibrary.CollectGarbage`))

(event `Update`
  (params (DeltaTime :type "Float (double-precision)"))
  (`self.UpdateAll` DeltaTime))

(fn `< Frame`
  (bind _returnvalue (- (`KismetMathLibrary.FTrunc` (`self.PlaybackFrame`)) 1))
  (set `self.PlaybackFrame` (`KismetMathLibrary.Conv_IntToDouble` _returnvalue))
  (set `self.PlaybackTime` (`TimeManagementBlueprintLibrary.Conv_QualifiedFrameTimeToSeconds` (make `QualifiedFrameTime` (make `FrameNumber` _returnvalue) (`MovieSceneSequencePlayer.GetFrameRate` (`self.SequencePlayer`)))))
  (`MovieSceneSequencePlayer.SetPlaybackPosition` (`self.SequencePlayer`) (make `MovieSceneSequencePlaybackParams` (make `FrameTime` (make `FrameNumber` _returnvalue)) 0.0 "" (struct) "Frame" "Jump"))
  (`self.UpdateTimeController`))

(fn `< Marker`
  (`/Engine/EditorBlueprintResources/StandardMacros.DecrementInt` (`self.Marker`)
    (:`  `
      (`self.Jump`))))

(fn `DisableCameraCuts`
  (params (Sequence :type "MovieSceneSequence Object Reference"))
  (bind _returnvalue (`MovieSceneSequenceExtensions.FindTracksByType` Sequence "/Script/MovieSceneTracks.MovieSceneCameraCutTrack"))
  (for _array_element _returnvalue
    (bind _returnvalue_2 (`MovieSceneTrackExtensions.GetSections` _array_element))
    (for _array_element_2 _returnvalue_2
      (bind _asmovie_scene_camera_cut_section (cast `MovieSceneCameraCutSection` _array_element_2))
      (if (`MovieSceneSection.IsActive` _asmovie_scene_camera_cut_section)
        (`MovieSceneSection.SetIsActive` _asmovie_scene_camera_cut_section false)
        (`KismetSystemLibrary.PrintString` (`KismetStringLibrary.Concat_StrStr` " \nTime Remapping disabled Camera Cuts in this sequence: " (`KismetSystemLibrary.GetObjectName` Sequence)) true true (struct :`R` 1.0 :`A` 1.0) 5.0)))))

(fn `DisableCameracutsAndTimecontrollers`
  (bind _returnvalue (`MovieSceneSequencePlayer.GetSequence` (`self.SequencePlayer`)))
  (bind _returnvalue_2 (`MovieSceneSequenceExtensions.FindTracksByType` _returnvalue "/Script/MovieScene.MovieSceneSubTrack"))
  (for _array_element _returnvalue_2
    (bind _returnvalue_3 (`MovieSceneTrackExtensions.GetSections` _array_element))
    (for _array_element_2 _returnvalue_3
      (bind _asmovie_scene_sub_section (cast `MovieSceneSubSection` _array_element_2))
      (bind _returnvalue_4 (`MovieSceneSubSection.GetSequence` _asmovie_scene_sub_section))
      (if (`KismetStringLibrary.Contains` (`KismetSystemLibrary.GetObjectName` _returnvalue_4) "TimeController")
        (if (`MovieSceneSection.IsActive` _asmovie_scene_sub_section)
          (`MovieSceneSection.SetIsActive` _asmovie_scene_sub_section false)
          (`KismetSystemLibrary.PrintString` (`KismetStringLibrary.Concat_StrStr` " \nTime Remapping disabled Time Controllers in this sequence: " (`KismetSystemLibrary.GetObjectName` _returnvalue)) true true (struct :`R` 1.0 :`B` 1.0 :`A` 1.0) 5.0))
        (else
          (`self.DisableCameraCuts` _returnvalue_4)))))
  (`self.DisableCameraCuts` _returnvalue))

(fn `Frame >`
  (bind _returnvalue (+ (`KismetMathLibrary.FTrunc` (`self.PlaybackFrame`)) 1))
  (set `self.PlaybackFrame` (`KismetMathLibrary.Conv_IntToDouble` _returnvalue))
  (set `self.PlaybackTime` (`TimeManagementBlueprintLibrary.Conv_QualifiedFrameTimeToSeconds` (make `QualifiedFrameTime` (make `FrameNumber` _returnvalue) (`MovieSceneSequencePlayer.GetFrameRate` (`self.SequencePlayer`)))))
  (`MovieSceneSequencePlayer.SetPlaybackPosition` (`self.SequencePlayer`) (make `MovieSceneSequencePlaybackParams` (make `FrameTime` (make `FrameNumber` _returnvalue)) 0.0 "" (struct) "Frame" "Jump"))
  (`self.UpdateTimeController`))

(fn `Jump`
  (bind _marker (`self.Marker`))
  (bind _returnvalue (`MovieSceneSequenceExtensions.GetMarkedFramesFromSequence` (`self.ActiveSequence`)))
  (if (`KismetArrayLibrary.Array_IsEmpty` _returnvalue)
    (`KismetSystemLibrary.PrintString` "No Marked Frames" true false (struct :`R` 1.0 :`A` 1.0))
    (else
      (bind _returnvalue_2 (`KismetArrayLibrary.Array_Length` _returnvalue))
      (if (or (< _marker 1) (> _marker _returnvalue_2))
        (set `self.Marker` (`KismetMathLibrary.SelectInt` 1 _returnvalue_2 (< (`self.Marker`) 1))))
      (bind _output (`|GetArrayItem` _returnvalue (- (`self.Marker`) 1)))
      (set `self.PlaybackFrame` (`KismetMathLibrary.Conv_IntToDouble` (break `FrameNumber` (break `MovieSceneMarkedFrame` _output))))
      (set `self.PlaybackTime` (`TimeManagementBlueprintLibrary.Conv_QualifiedFrameTimeToSeconds` (make `QualifiedFrameTime` (make `FrameNumber` (break `FrameNumber` (break `MovieSceneMarkedFrame` _output))) (`MovieSceneSequencePlayer.GetFrameRate` (`self.SequencePlayer`)))))
      (`MovieSceneSequencePlayer.SetPlaybackPosition` (`self.SequencePlayer`) (make `MovieSceneSequencePlaybackParams` (make `FrameTime` (make `FrameNumber` (break `FrameNumber` (break `MovieSceneMarkedFrame` _output)))) 0.0 "" (struct) "Frame" "Jump"))
      (`self.UpdateTimeController`))))

(fn `Marker >`
  (`/Engine/EditorBlueprintResources/StandardMacros.IncrementInt` (`self.Marker`)
    (:`  `
      (`self.Jump`))))

(fn `RefreshActorsList`
  (if (`self.AutoAddActors`)
    (for _array_element (`self.ActorClass`)
      (bind _outactors (`GameplayStatics.GetAllActorsOfClass` _array_element))
      (for _array_element_2 _outactors
        (`KismetArrayLibrary.Array_AddUnique` (`self.Actors`) _array_element_2)))))

(fn `ResetParticlesAndMaterials`
  (for _array_element (`self.Actors`)
    (`|ExecutionSequence`
      (:`then_0`
        (set `Actor.CustomTimeDilation` 1.0 _array_element))
      (:`then_1`
        (`self.SetNiagaraTimeDilation` _array_element))
      (:`then_2`
        (`self.SetCascadeTimeDilation` _array_element))))
  (`KismetMaterialLibrary.SetScalarParameterValue` (`self.MpcRemappedTime`) "Enabled"))

(fn `SetCascadeTimeDilation`
  (params (Actor :type "Actor Object Reference") (Dilation :type "Float (single-precision)" :default 1.0))
  (bind _returnvalue (`self.K2_GetComponentsByClass` Actor "/Script/Engine.ParticleSystemComponent"))
  (if (`KismetArrayLibrary.Array_IsNotEmpty` _returnvalue)
    (for _array_element _returnvalue
      (set `ParticleSystemComponent.CustomTimeDilation` Dilation _array_element))))

(fn `SetCustomTimeDilationNiagara_Old`
  (params (NiagaraComponent :type "NiagaraComponent Object Reference"))
  (`NiagaraComponent.SetPaused` NiagaraComponent false)
  (`NiagaraComponent.AdvanceSimulation` NiagaraComponent 1 (`KismetMathLibrary.Abs` 0.0))
  (`NiagaraComponent.SetPaused` NiagaraComponent true))

(fn `SetNiagaraTimeDilation`
  (params (Actor :type "Actor Object Reference") (Dilation :type "Float (single-precision)" :default 1.0))
  (bind _returnvalue (`self.K2_GetComponentsByClass` Actor "/Script/Niagara.NiagaraComponent"))
  (if (`KismetArrayLibrary.Array_IsNotEmpty` _returnvalue)
    (for _array_element _returnvalue
      (`NiagaraComponent.SetCustomTimeDilation` _array_element Dilation))))

(fn `SetSequenceDeltaSeconds`
  (params (DeltaSeconds :type "Float (double-precision)"))
  (set `self.SequenceDeltaSeconds` (/ (- (`self.PlaybackTime`) (`self.PreviousPlaybackTIme`)) DeltaSeconds))
  (set `self.PreviousPlaybackTIme` (`self.PlaybackTime`)))

(fn `Stop`
  (`MovieSceneSequencePlayer.GoToEndAndStop` (`self.SequencePlayer`)))

(fn `UpdateAll`
  (params (DeltaTime :type "Float (double-precision)"))
  (bind _returnvalue (`MovieSceneSequencePlayer.GetCurrentTime` (`self.SequencePlayer`)))
  (`self.SetSequenceDeltaSeconds` DeltaTime)
  (if (`self.Active`)
    (`/Engine/EditorBlueprintResources/StandardMacros.IsValid` (`self.ActiveSequence`)
      (:`Is Valid`
        (if (not (and (== (`self.SequenceCheck`) (`self.ActiveSequence`)) (`KismetSystemLibrary.IsValid` (`self.GetSequence` self))))
          (set `self.SequenceCheck` (`self.ActiveSequence`))
          (`self.SetSequence` (`self.ActiveSequence`))
          (`self.DisableCameracutsAndTimecontrollers`))
        (`|ExecutionSequence`
          (:`then_0`
            (if (`self.UseFrame`)
              (`MovieSceneSequencePlayer.SetPlaybackPosition` (`self.SequencePlayer`) (make `MovieSceneSequencePlaybackParams` (make `FrameTime` (make `FrameNumber` (`KismetMathLibrary.FTrunc` (`self.PlaybackFrame`))) (`KismetMathLibrary.Fraction` (`self.PlaybackFrame`)))))
              (set `self.PlaybackTime` (`TimeManagementBlueprintLibrary.Conv_QualifiedFrameTimeToSeconds` (`MovieSceneSequencePlayer.GetCurrentTime` (`self.SequencePlayer`))))
              (else
                (`MovieSceneSequencePlayer.SetPlaybackPosition` (`self.SequencePlayer`) (make `MovieSceneSequencePlaybackParams` (struct :`FrameNumber` (struct)) (+ (`self.PlaybackTime`) 1e-05) "" (struct) "Time"))
                (set `self.PlaybackFrame` (+ (`KismetMathLibrary.Conv_IntToDouble` (break `FrameNumber` (break `QualifiedFrameTime` _returnvalue))) (`.SubFrame` (break `QualifiedFrameTime` _returnvalue)))))))
          (:`then_1`
            (`|ExecutionSequence`
              (:`then_0`
                (for _array_element (`self.Actors`)
                  (`|ExecutionSequence`
                    (:`then_0`
                      (set `Actor.CustomTimeDilation` (`KismetMathLibrary.Abs` (`self.SequenceDeltaSeconds`)) _array_element))
                    (:`then_1`
                      (`self.SetNiagaraTimeDilation` _array_element (`KismetMathLibrary.Abs` (`self.SequenceDeltaSeconds`))))
                    (:`then_2`
                      (`self.SetCascadeTimeDilation` _array_element (`KismetMathLibrary.Abs` (`self.SequenceDeltaSeconds`)))))))
              (:`then_1`
                (if (`self.EnableMaterials`)
                  (`KismetMaterialLibrary.SetScalarParameterValue` (`self.MpcRemappedTime`) "Enabled" 1.0)
                  (`KismetMaterialLibrary.SetScalarParameterValue` (`self.MpcRemappedTime`) "Time" (`self.PlaybackTime`)))))))))))

(fn `UpdateTimeController`
  (bind _returnvalue (`GameplayStatics.GetActorOfClass` "/Game/_kitmvm/Blueprints/Editing/Resources/TimeController.TimeController_C"))
  (`/Engine/EditorBlueprintResources/StandardMacros.IsValid` _returnvalue
    (:`Is Valid`
      (`/Game/_kitmvm/Blueprints/Editing/Resources/TimeController.UpdateCustom` _returnvalue 0.04))))

(fn `UserConstructionScript`
  (`self.RefreshActorsList`)
  (`self.UpdateTimeController`))