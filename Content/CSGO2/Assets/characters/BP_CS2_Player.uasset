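; CS2 player character Blueprint that assembles its appearance by merging modular skeletal meshes.
; UET Merge looks up ModelName in DT_CharacterConfig and synchronously loads body, gloves and skintone material, then calls Merge.
; Merge combines body, gloves and optional defuse kit on the shared master skeleton, then applies the skintone to the bare_arm slot.
; BeginPlay and the construction script do nothing, so merging only runs when called.
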(event `self.ReceiveBeginPlay`)

(fn `Merge`
  (locals (NewLocalVar :type "Array of SkeletalMaterial Structure"))
  (bind _meshes_to_merge (`self.Meshes To Merge`))
  (bind _skeletalmeshcomponent (`self.SkeletalMeshComponent`))
  (bind _skintone (`self.Skintone`))
  (bind _returnvalue (`PrimitiveComponent.GetMaterialIndex` _skeletalmeshcomponent "bare_arm"))
  (`KismetArrayLibrary.Array_Append` _meshes_to_merge (`|MakeArray` (`self.Body`) (`self.Gloves`)))
  (if (`self.Defuse kits`)
    (`KismetArrayLibrary.Array_Add` _meshes_to_merge "/Game/CSGO2/Assets/characters/shared/defuse_kits.defuse_kits"))
  (bind _returnvalue_2 (`self.MergeMeshes` (make `` (`self.Meshes To Merge`) "/Game/CSGO2/Assets/characters/CSGO2_Players_MasterSkeleton.CSGO2_Players_MasterSkeleton")))
  (`/Engine/EditorBlueprintResources/StandardMacros.IsValid` _returnvalue_2
    (:`Is Valid`
      (`SkeletalMeshComponent.SetSkeletalMeshAsset` _skeletalmeshcomponent _returnvalue_2)
      (`/Engine/EditorBlueprintResources/StandardMacros.IsValid` _skintone
        (:`Is Valid`
          (if (!= _returnvalue -1)
            (`PrimitiveComponent.SetMaterial` _skeletalmeshcomponent _returnvalue _skintone)))))))

(fn `UET Merge`
  (locals (NewLocalVar :type "Array of SkeletalMaterial Structure"))
  (bind _returnvalue (`|GetDataTableRow` "/Game/CSGO2/Assets/characters/data/DT_CharacterConfig.DT_CharacterConfig" (`KismetStringLibrary.Conv_StringToName` (`self.ModelName`)))
    (:`then`
      (`|ExecutionSequence`
        (:`then_0`
          (bind _returnvalue_2 (`KismetSystemLibrary.LoadAsset_Blocking` (`.Body_10_4915558E4E57B6980FBBE0A77A9B96E0` (break `/Game/CSGO2/Assets/characters/data/S_CharacterConfig` _returnvalue))))
          (`/Engine/EditorBlueprintResources/StandardMacros.IsValid` _returnvalue_2
            (:`Is Valid`
              (bind _asskeletal_mesh (cast `SkeletalMesh` _returnvalue_2))
              (set `self.Body` _asskeletal_mesh))))
        (:`then_1`
          (bind _returnvalue_3 (`KismetSystemLibrary.LoadAsset_Blocking` (`.Gloves_11_73C178AE464236561D8C5691B708CF81` (break `/Game/CSGO2/Assets/characters/data/S_CharacterConfig` _returnvalue))))
          (`/Engine/EditorBlueprintResources/StandardMacros.IsValid` _returnvalue_3
            (:`Is Valid`
              (bind _asskeletal_mesh_2 (cast `SkeletalMesh` _returnvalue_3))
              (set `self.Gloves` _asskeletal_mesh_2))))
        (:`then_2`
          (bind _returnvalue_4 (`KismetSystemLibrary.LoadAsset_Blocking` (`.SkintoneMaterial_12_3DF0ADBB4E35889FE00D7C9EDDCD6065` (break `/Game/CSGO2/Assets/characters/data/S_CharacterConfig` _returnvalue))))
          (`/Engine/EditorBlueprintResources/StandardMacros.IsValid` _returnvalue_4
            (:`Is Valid`
              (bind _asmaterial_instance (cast `MaterialInstance` _returnvalue_4))
              (set `self.Skintone` _asmaterial_instance))))
        (:`then_3`
          (`self.Merge`))))))

(fn `UserConstructionScript`)