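; VisibilityActor is a grouping actor that controls the visibility of the actors and components attached beneath it.
; On construction, it makes a designated actor the owner of all attached actors and applies owner-see and hidden-shadow settings to their primitives, resetting those flags without one.
; Hide and Unhide propagate visibility through the root's children, then update attached VisibilityActors, which combine their own state with the received parent flag.
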(event `Update`
  (`self.SetVisibility`))

(fn `ActorVisibility`
  (params (Reset :type Boolean))
  (locals (ActorsToConfigure :type "Array of Actor Object Reference"))
  (for _array_element (`self.GetAttachedActors` true true)
    (if (!= _array_element (`self.OwnerOfActors (Hover over for desc)`))
      (if (not (`local.Reset`))
        (`self.SetOwner` _array_element (`self.OwnerOfActors (Hover over for desc)`)))
      (for _array_element_2 (`self.K2_GetComponentsByClass` _array_element "/Script/Engine.PrimitiveComponent")
        (`PrimitiveComponent.SetOnlyOwnerSee` _array_element_2 (select `bool` (`local.Reset`) :`false` (`self.OnlyOwnerSee`)))
        (`PrimitiveComponent.SetOwnerNoSee` _array_element_2 (select `bool` (`local.Reset`) :`false` (`self.OwnerNoSee`)))
        (`PrimitiveComponent.SetCastHiddenShadow` _array_element_2 (select `bool` (`local.Reset`) :`false` (`self.HiddenShadow`)))))))

(fn `Hide`
  (set `self.Visibility` false)
  (`self.SetVisibility`))

(fn `SetVisibility`
  (`|ExecutionSequence`
    (:`then_0`
      (`SceneComponent.SetVisibility` (`self.DefaultSceneRoot`) (and (`self.Visibility`) (`self.ParentVisibility`)) true))
    (:`then_1`
      (bind _filteredarray (`KismetArrayLibrary.FilterArray` (`self.GetAttachedActors` true true) "VisibilityActor_C"))
      (for _array_element _filteredarray
        (set `/Game/_kitmvm/Blueprints/Editing/VisibilityActor.ParentVisibility` (`self.Visibility`) _array_element)
        (`self.Update` _array_element)))))

(fn `Unhide`
  (set `self.Visibility` true)
  (`self.SetVisibility`))

(fn `UserConstructionScript`
  (`/Engine/EditorBlueprintResources/StandardMacros.IsValid` (`self.OwnerOfActors (Hover over for desc)`)
    (:`Is Valid`
      (`self.ActorVisibility` false))
    (:`Is Not Valid`
      (`self.ActorVisibility` true))))