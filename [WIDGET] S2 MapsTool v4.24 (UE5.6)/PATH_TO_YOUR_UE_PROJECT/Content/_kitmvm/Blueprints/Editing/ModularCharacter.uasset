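; Modular character actor that assembles its look from a list of skeletal mesh modules in the Construction Script.
; Each module becomes a new component snapped to the main skeletal mesh, with optional per-slot material overrides applied.
; Modules use the main mesh as leader pose, so they follow its animation, and take a shared bounds scale plus its owner visibility flags.
; The Event Graph has no active logic.
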(fn `UserConstructionScript`
  (for _array_element (`self.Modules`)
    (bind _returnvalue (`AddComponent|NODE_AddSkeletalMeshComponent-0` :`bManualAttachment` true))
    (`SceneComponent.K2_AttachToComponent` _returnvalue (`self.SkeletalMeshComponent`) "None" "SnapToTarget" "SnapToTarget" "SnapToTarget" true)
    (`SkeletalMeshComponent.SetSkeletalMeshAsset` _returnvalue (break `/Game/_kitmvm/Blueprints/Editing/Resources/S_ModularCharacter_Module` _array_element))
    (`SkinnedMeshComponent.SetLeaderPoseComponent` _returnvalue (`self.SkeletalMeshComponent`) true true)
    (for (_array_element_2 _array_index) (`.MaterialsOverrides_7_D10C426446232ABAD8A941869D51EFC7` (break `/Game/_kitmvm/Blueprints/Editing/Resources/S_ModularCharacter_Module` _array_element))
      (`/Engine/EditorBlueprintResources/StandardMacros.IsValid` _array_element_2
        (:`Is Valid`
          (`PrimitiveComponent.SetMaterial` _returnvalue _array_index _array_element_2))))
    (`PrimitiveComponent.SetBoundsScale` _returnvalue (`self.ModulesBoundsScale`))
    (`PrimitiveComponent.SetOwnerNoSee` _returnvalue (`PrimitiveComponent.bOwnerNoSee` (`self.SkeletalMeshComponent`)))
    (`PrimitiveComponent.SetOnlyOwnerSee` _returnvalue (`PrimitiveComponent.bOnlyOwnerSee` (`self.SkeletalMeshComponent`)))))